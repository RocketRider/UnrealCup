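; Ball Blueprint that exposes an event for pushing the ball with a physics impulse.
; AddImpulseBlueprint scales Direction by Force, applies it as a velocity change so mass is ignored, and prints the vector for debugging.
; A Clamp helper tests against symmetric limits but is unfinished: it never substitutes a limit value and is not called in these graphs.
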(event EventAddImpulseBlueprint
  (params (direction :type Vector :default "0, 0, 0") (force :type Float%20%28single-precision%29))
  (bind _returnvalue (* direction force))
  (Physics|AddImpulse self _returnvalue "None" true)
  (Development|PrintString (Utilities|String|ToString(Vector) _returnvalue) true true "(R=1.000000,G=0.020153,B=0.251691,A=1.000000)"))

(fn ConstructionScript)

(fn Clamp
  (params (in :type Float%20%28single-precision%29))
  (if (>= in 1e+04)
    _
    (else
      _))
  (if (not (<= in -1e+04))
    (return in)))