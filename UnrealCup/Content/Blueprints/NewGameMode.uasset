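; Game mode Blueprint that keeps the score and names for a two-team, goal-based match.
; BeginPlay resets both scores to zero and sets hardcoded placeholder team names, with a TODO about possibly loading them from XML.
; Separate goal functions increment each team's score by one, and getter functions expose names and scores to other Blueprints.
; It contains no win condition or other match-flow logic.
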(event EventBeginPlay
  ;[1 1 1] Spielstand initialisieren...
  (Variables|Default|SetScoreTeam1 0)
  (Variables|Default|SetScoreTeam2 0)
  ;[1 1 1] TODO: Namen der Teams aus XML?
  (Variables|Default|SetNameTeam1 "Team1")
  (Variables|Default|SetNameTeam2 "Team2"))

(fn ConstructionScript)

(fn GoalTeam1
  (Variables|Default|SetScoreTeam1 (+ (Variables|Default|GetScoreTeam1) 1)))

(fn GoalTeam2
  (Variables|Default|SetScoreTeam2 (+ (Variables|Default|GetScoreTeam2) 1)))

(fn GetNameTeam1
  (return (Variables|Default|GetNameTeam1)))

(fn GetNameTeam2
  (return (Variables|Default|GetNameTeam2)))

(fn GetScoreTeam1
  (return (Variables|Default|GetScoreTeam1)))

(fn GetScoreTeam2
  (return (Variables|Default|GetScoreTeam2)))