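; Soccer ball Blueprint that takes physics impulses and tracks whether a kickoff is in progress.
; Setting kickoff state starts or clears a short timer; on expiry, RemovePlayers tells the SoccerLevelScript to send a kickoff signal and check players.
; Reset returns the ball to a fixed point above the origin and zeroes linear and angular velocity on its primitive components.
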(event EventAddImpulseBlueprint
  (params (direction :type Vector :default "0, 0, 0") (force :type Float%20%28single-precision%29))
  (Physics|AddImpulse (* direction force) "None" false))

(event EventSetKickoffState
  (params (state :type Boolean))
  (bind _output_get (Variables|Default|SetisKickoff state))
  (if _output_get
    (Utilities|Time|SetTimerbyFunctionName 0 "removePlayers" 3.0)
    (else
      (Utilities|Time|ClearTimerbyFunctionName 0 "removePlayers"))))

(fn ConstructionScript)

(fn Clamp
  (params (in :type Float%20%28single-precision%29))
  (if (>= in 1e+04)
    _
    (else
      _))
  (if (not (<= in -1e+04))
    (return in)))

(fn Reset
  (Transformation|SetActorLocation "0, 0,300.000000" false)
  (for _array_element (Actor|GetComponentsByClass "/Script/Engine.PrimitiveComponent")
    (bind _asprimitive_component (Utilities|Casting|CastToPrimitiveComponent _array_element))
    (Class|PrimitiveComponent|SetAllPhysicsLinearVelocity _asprimitive_component "0, 0, 0" false)
    (Class|PrimitiveComponent|SetPhysicsAngularVelocity _asprimitive_component "0, 0, 0" false "None")))

(fn RemovePlayers
  (if (Variables|Default|GetisKickoff)
    (bind _outactors (Actor|GetAllActorsOfClass "/Script/UnrealCup.SoccerLevelScript"))
    (Class|SoccerLevelScript|SendKickoff (Utilities|Array|Get(acopy) _outactors) -1)
    (Class|SoccerLevelScript|CheckPlayers (Utilities|Array|Get(acopy) _outactors))))