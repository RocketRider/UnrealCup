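; Robot pawn that can halt a ball within its range and move via AI navigation.
; BallRange overlaps track BallInRange, which the stopBallNow event checks before immediately stopping every movement component on Ball1.
; An actor named "Ball" entering the range within a second of StopCommandTime triggers the same stop, allowing slightly early commands.
; A separate moveToLoc event calls SimpleMoveToLocation on the robot's controller.
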(event OnComponentBeginOverlap(BallRange)
  (params (OtherActor :type Actor%20Object%20Reference) (OtherComp :type Primitive%20Component%20Object%20Reference) (OtherBodyIndex :type Integer) (bFromSweep :type Boolean) (SweepResult :type Hit%20Result%20Structure%20%28by%20ref%29))
  (Variables|Default|SetballInRange true)
  (if (Utilities|Enum|Equal(Enum) (Utilities|GetDisplayName OtherActor) "Ball")
    (if (<= (Math|DateTime|Now) (+ (Variables|Default|GetstopCommandTime) (Math|Timespan|FromSeconds 1.0)))
      (for _array_element (Actor|GetComponentsByClass (Variables|Default|Getball1) "/Script/Engine.MovementComponent")
        (bind _asmovement_component (Utilities|Casting|CastToMovementComponent _array_element))
        (Components|Movement|StopMovementImmediately _asmovement_component)
        (Variables|Default|SettryStopBall false)))))

(event OnComponentEndOverlap(BallRange)
  (params (OtherActor :type Actor%20Object%20Reference) (OtherComp :type Primitive%20Component%20Object%20Reference) (OtherBodyIndex :type Integer))
  (Variables|Default|SetballInRange false))

(event Custom|moveToLoc
  (AI|Navigation|SimpleMovetoLocation (Pawn|GetController) "0, 0, 0"))

(event Custom|stopBallNow
  (if (Variables|Default|GetballInRange)
    (for _array_element (Actor|GetComponentsByClass (Variables|Default|Getball1) "/Script/Engine.MovementComponent")
      (bind _asmovement_component (Utilities|Casting|CastToMovementComponent _array_element))
      (Components|Movement|StopMovementImmediately _asmovement_component)
      (Variables|Default|SettryStopBall false))))

(fn ConstructionScript)