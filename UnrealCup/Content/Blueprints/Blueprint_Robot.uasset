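; Robot character for a team-based ball game that moves to commanded locations and can stop the ball.
; MovetoLoc sets walk speed and uses SimpleMoveToLocation, while BallRange overlaps track the ball by display name.
; StopBallNow zeroes every Blueprint_Ball's velocity when one is in range; the delayed-stop retry is left unconnected.
; The construction script applies the Team1 material for team 1.
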(event OnComponentBeginOverlap(BallRange)
  (params (OtherActor :type Actor%20Object%20Reference) (OtherComp :type Primitive%20Component%20Object%20Reference) (OtherBodyIndex :type Integer) (bFromSweep :type Boolean) (SweepResult :type Hit%20Result%20Structure%20%28by%20ref%29))
  (if (Utilities|Enum|Equal(Enum) (Utilities|GetDisplayName OtherActor) "Ball")
    (Variables|Default|SetballInRange true)
    (if (Variables|Default|GettryStopBall)
      _)))

(event OnComponentEndOverlap(BallRange)
  (params (OtherActor :type Actor%20Object%20Reference) (OtherComp :type Primitive%20Component%20Object%20Reference) (OtherBodyIndex :type Integer))
  (if (Utilities|Enum|Equal(Enum) (Utilities|GetDisplayName OtherActor) "Ball")
    (Variables|Default|SetballInRange false)))

(event EventMovetoLoc
  (params (location :type Vector :default "0, 0, 0") (speed :type Float%20%28single-precision%29))
  (Variables|/Script/Engine.CharacterMovementComponent|SetMaxWalkSpeed (Variables|Character|GetCharacterMovement) speed)
  (AI|Navigation|SimpleMovetoLocation (Pawn|GetController) location))

(event EventStopBallNow
  (if (Variables|Default|GetballInRange)
    (bind _outactors (Actor|GetAllActorsOfClass "/Game/Blueprints/Blueprint_Ball.Blueprint_Ball_C"))
    (for _array_element _outactors
      (Class|PrimitiveComponent|SetAllPhysicsLinearVelocity (Variables|/Game/Blueprints/Blueprint_Ball.Blueprint_Ball_C|GetStaticMesh1 _array_element) "0, 0, 0" false)
      (Class|PrimitiveComponent|SetPhysicsAngularVelocity (Variables|/Game/Blueprints/Blueprint_Ball.Blueprint_Ball_C|GetStaticMesh1 _array_element) "0, 0, 0" false "None")
      (Variables|Default|SettryStopBall false))))

(fn ConstructionScript
  (if (== 1 (Variables|Default|Getteam))
    (Rendering|Material|SetMaterial 0 "/Game/Props/Team1.Team1")))